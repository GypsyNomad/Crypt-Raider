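; BP_Player is the player Blueprint that lets the player grab, release and open things.
; On BeginPlay it adds the Interaction mapping context to the local player's Enhanced Input subsystem, provided its controller is a PlayerController.
; GrabAction tells the Grabber to grab when it starts and release when it completes, while OpenAction asks the Opener to try opening, leaving the interaction logic to those two objects.
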(event `self.ReceiveBeginPlay`
  (bind _asplayer_controller (cast `PlayerController` (`self.GetController`)))
  (message `EnhancedInputSubsystemInterface.AddMappingContext` (pcsubsystem `EnhancedInputLocalPlayerSubsystem` _asplayer_controller) "/Game/Interaction.Interaction" 0 (struct)))

(event `EnhancedInput|/Game/GrabAction`
  (params (ActionValue :type Boolean) (ElapsedSeconds :type "Float (double-precision)") (TriggeredSeconds :type "Float (double-precision)") (InputAction :type "InputAction Object Reference" :default "/Game/GrabAction.GrabAction"))
  (bind _grabber (`self.Grabber`))
  (:`Started`
    (`Grabber.Grab` _grabber))
  (:`Completed`
    (`Grabber.Release` _grabber)))

(event `EnhancedInput|/Game/OpenAction`
  (params (ActionValue :type Boolean) (ElapsedSeconds :type "Float (double-precision)") (TriggeredSeconds :type "Float (double-precision)") (InputAction :type "InputAction Object Reference" :default "/Game/OpenAction.OpenAction"))
  (:`Triggered`
    (`Opener.TryOpen` (`self.Opener`))))

(fn `UserConstructionScript`
  (`parent.UserConstructionScript`))