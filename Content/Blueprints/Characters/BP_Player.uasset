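; BP_Player is the player character Blueprint, routing Enhanced Input actions for grabbing, opening and interacting.
; On BeginPlay it adds the IMC_Interaction mapping context to the player controller's Enhanced Input subsystem.
; The grab action drives the Grabber on press and release, while the open and interact actions call the Opener and Interactor.
; The construction script only calls the parent's.
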(event `self.ReceiveBeginPlay`
  (bind _asplayer_controller (cast `PlayerController` (`self.GetController`)))
  (message `EnhancedInputSubsystemInterface.AddMappingContext` (pcsubsystem `EnhancedInputLocalPlayerSubsystem` _asplayer_controller) "/Game/Blueprints/Input/IMC_Interaction.IMC_Interaction" 0 (struct)))

(event `EnhancedInput|/Game/Blueprints/Input/IA_Grab`
  (params (ActionValue :type Boolean) (ElapsedSeconds :type "Float (double-precision)") (TriggeredSeconds :type "Float (double-precision)") (InputAction :type "InputAction Object Reference" :default "/Game/Blueprints/Input/IA_Grab.IA_Grab"))
  (bind _grabber (`self.Grabber`))
  (:`Started`
    (`Grabber.Grab` _grabber))
  (:`Completed`
    (`Grabber.Release` _grabber)))

(event `EnhancedInput|/Game/Blueprints/Input/IA_Open`
  (params (ActionValue :type Boolean) (ElapsedSeconds :type "Float (double-precision)") (TriggeredSeconds :type "Float (double-precision)") (InputAction :type "InputAction Object Reference" :default "/Game/Blueprints/Input/IA_Open.IA_Open"))
  (:`Triggered`
    (`Opener.TryOpen` (`self.Opener`))))

(event `EnhancedInput|/Game/Blueprints/Input/IA_Interact`
  (params (ActionValue :type Boolean) (ElapsedSeconds :type "Float (double-precision)") (TriggeredSeconds :type "Float (double-precision)") (InputAction :type "InputAction Object Reference" :default "/Game/Blueprints/Input/IA_Interact.IA_Interact"))
  (:`Triggered`
    (`Interactor.TryInteract` (`self.Interactor`))))

(fn `UserConstructionScript`
  (`parent.UserConstructionScript`))